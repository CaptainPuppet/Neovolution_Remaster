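; TextTestTrigger is a proximity trigger that reveals TextTest widgets when the player presses F.
; On BeginPlay it hides all TextTest widgets found through GetAllWidgetsOfClass.
; Overlap of Sphere1 by a ThirdPersonCharacter sets the Esenrango in-range flag, which lets F show those widgets.
; The logic to clear the flag and re-hide them is disconnected, so both persist once set, and debug prints remain.
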(event OnComponentBeginOverlap(Sphere1)
  (params (OverlappedComponent :type Primitive%20Component%20Object%20Reference) (OtherActor :type Actor%20Object%20Reference) (OtherComp :type Primitive%20Component%20Object%20Reference) (OtherBodyIndex :type Integer) (bFromSweep :type Boolean) (SweepResult :type Hit%20Result%20Structure%20%28by%20ref%29))
  (Utilities|Casting|CastToThirdPersonCharacter OtherActor)
  (Variables|Default|Setesenrango true)
  (Development|PrintString "activado"))

(event EventBeginPlay
  (bind _foundwidgets (Widget|GetAllWidgetsOfClass "/Game/NEOVOLUTION/Blueprints/Widgets/UI/TextTest.TextTest_C" false))
  (Widget|SetVisibility _foundwidgets "Hidden"))

(event Collision|EventActorBeginOverlap
  (params (OtherActor :type Actor%20Object%20Reference)))

(event EventTick
  (params (DeltaSeconds :type Float%20%28single-precision%29)))

(event Input|KeyboardEvents|F
  (params (Key :type Key%20Structure :default "None"))
  (:Pressed
    (if (Variables|Default|Getesenrango)
      (Development|PrintString "pinchi unreal")
      (bind _foundwidgets (Widget|GetAllWidgetsOfClass "/Game/NEOVOLUTION/Blueprints/Widgets/UI/TextTest.TextTest_C" false))
      (Widget|SetVisibility _foundwidgets "Visible"))))

(fn ConstructionScript)