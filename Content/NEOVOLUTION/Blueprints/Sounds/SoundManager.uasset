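; SoundManager switches the background music to match the game state, covering menu, pause/skills, level, cinematics, combat and boss fights.
; ChangeMusic maps the state to a track, caching level and combat tracks in TempSound to restore when leaving menu, pause or skills.
; If the AudioComponent, initially set from Audio on BeginPlay, is valid and the track differs, it stops it and spawns a replacement 2D sound that persists across level transitions.
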(event Custom|ChangeMusic
  (params (State :type PlayerSoundState%20Enum :default "NewEnumerator0"))
  (switch Utilities|FlowControl|Switch|SwitchonPlayerSoundState State
    (:NewEnumerator0
      (Variables|Default|SetSound "/Game/NEOVOLUTION/Music_Sounds/Music/Adventure.Adventure"))
    (:NewEnumerator6
      (Variables|Default|SetSound "/Game/NEOVOLUTION/Music_Sounds/Music/dub-techno-loop-01-1589.dub-techno-loop-01-1589"))
    (:NewEnumerator1
      (bind _output_get (Variables|Default|SetSound "/Game/NEOVOLUTION/Music_Sounds/Music/thinking-time-148496.thinking-time-148496"))
      (Variables|Default|SetTempSound _output_get))
    (:NewEnumerator2
      (Variables|Default|SetSound "/Game/NEOVOLUTION/Music_Sounds/Music/Celestial__CC-BY_.Celestial__CC-BY_"))
    (:NewEnumerator3
      (Variables|Default|SetSound "/Game/NEOVOLUTION/Music_Sounds/Music/Our_Forbidden_Role.Our_Forbidden_Role"))
    (:NewEnumerator4
      (bind _output_get_2 (Variables|Default|SetSound "/Game/NEOVOLUTION/Music_Sounds/Music/Crux.Crux"))
      (Variables|Default|SetTempSound _output_get_2))
    (:NewEnumerator5
      (bind _output_get_3 (Variables|Default|SetSound "/Game/NEOVOLUTION/Music_Sounds/Music/background-loop-funky-04-3515.background-loop-funky-04-3515"))
      (Variables|Default|SetTempSound _output_get_3))
    (:NewEnumerator7
      (Variables|Default|SetSound (Variables|Default|GetTempSound))))
  (Utilities|IsValid (Variables|Default|GetAudioComponent)
    (:Is%20Valid
      (if (not (== (Variables|/Script/Engine.AudioComponent|GetSound (Variables|Default|GetAudioComponent)) (Variables|Default|GetSound)))
        (Audio|Components|Audio|Stop (Variables|Default|GetAudioComponent))
        (bind _returnvalue (Audio|SpawnSound2D (Variables|Default|GetSound) 0.25 1.0 0.0 0 true))
        (Variables|Default|SetAudioComponent _returnvalue)))))

(event EventBeginPlay
  (Variables|Default|SetAudioComponent (Variables|Default|GetAudio)))

(fn ConstructionScript)