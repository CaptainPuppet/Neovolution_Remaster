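; Statue puzzle window that opens and teleports the player once the arms, feet, torsos and heads collected flags are all set.
; Trigger overlap adds an audio component, shrinks and raises the mesh for ThirdPersonCharacter, waits briefly, then moves it to the Arrow.
; For the player, it also aligns control rotation and zeroes velocity; ending overlap restores the mesh.
; The construction script places the Arrow from TPLocation; UpdateLight is empty.
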(event OnComponentBeginOverlap(DoorTrigger)
  (params (OverlappedComponent :type Primitive%20Component%20Object%20Reference) (OtherActor :type Actor%20Object%20Reference) (OtherComp :type Primitive%20Component%20Object%20Reference) (OtherBodyIndex :type Integer) (bFromSweep :type Boolean) (SweepResult :type Hit%20Result%20Structure%20%28by%20ref%29))
  (bind _returnvalue (Game|GetPlayerCharacter 0))
  (bind _arrow (Variables|Default|GetArrow))
  (bind _returnvalue_2 (Transformation|GetWorldTransform _arrow))
  (if (and (and (Variables|Default|GetarmsCollected) (Variables|Default|GetfeetCollected)) (and (Variables|Default|GettorsosCollected) (Variables|Default|GetheadsCollected)))
    (bind _returnvalue_3 (AddComponent|AddAudioComponent false))
    (Variables|Default|SetsoundCue _returnvalue_3)
    (Utilities|Casting|CastToThirdPersonCharacter OtherActor)
    (Transformation|SetRelativeScale3D (Variables|Default|GetWindowMesh) "1.000000,0.100000,0.400000")
    (Transformation|SetRelativeLocation (Variables|Default|GetWindowMesh) "0, 0,180.000000" false false)
    (Utilities|FlowControl|Delay 0.5)
    (Transformation|SetWorldTransform (Variables|/Script/Engine.Actor|GetRootComponent OtherActor) (Math|Transform|MakeTransform (.location _returnvalue_2) (.rotation _returnvalue_2) "1,1,1") false false)
    (if (== _returnvalue OtherActor)
      (Pawn|SetControlRotation (Game|GetPlayerController 0) (Transformation|GetActorRotation _returnvalue))
      (Variables|/Script/Engine.MovementComponent|SetVelocity (Variables|/Script/Engine.Character|GetCharacterMovement _returnvalue) "0, 0, 0"))))

(event OnComponentEndOverlap(DoorTrigger)
  (params (OverlappedComponent :type Primitive%20Component%20Object%20Reference) (OtherActor :type Actor%20Object%20Reference) (OtherComp :type Primitive%20Component%20Object%20Reference) (OtherBodyIndex :type Integer))
  (Utilities|Casting|CastToThirdPersonCharacter OtherActor)
  (Transformation|SetRelativeScale3D (Variables|Default|GetWindowMesh) "1.000000,0.100000,2.000000")
  (Transformation|SetRelativeLocation (Variables|Default|GetWindowMesh) "0, 0,90.000000" false false))

(event EventBeginPlay)

(event Collision|EventActorBeginOverlap
  (params (OtherActor :type Actor%20Object%20Reference)))

(event EventTick
  (params (DeltaSeconds :type Float%20%28single-precision%29)))

(fn ConstructionScript
  (Transformation|SetRelativeTransform (Variables|Default|GetArrow) (Variables|Default|GetTP_Location) false false))

(fn UpdateLight)