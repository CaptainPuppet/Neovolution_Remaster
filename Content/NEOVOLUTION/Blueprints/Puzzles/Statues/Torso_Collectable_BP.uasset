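; Collectable statue torso for the statues puzzle, picked up with F while the ThirdPersonCharacter is inside its collision.
; Overlap begin and end toggle the actor's input for player 0.
; Pickup increments the game mode's torso counters, flags the torso as collected on StatuesWindow_BP, and shows a widget with a sound.
; It then spawns Torso_Spawnable_BP at a hardcoded world transform and destroys itself.
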(event OnComponentBeginOverlap(Collision)
  (params (OverlappedComponent :type Primitive%20Component%20Object%20Reference) (OtherActor :type Actor%20Object%20Reference) (OtherComp :type Primitive%20Component%20Object%20Reference) (OtherBodyIndex :type Integer) (bFromSweep :type Boolean) (SweepResult :type Hit%20Result%20Structure%20%28by%20ref%29))
  (Utilities|Casting|CastToThirdPersonCharacter OtherActor)
  (Input|EnableInput (Game|GetPlayerController 0)))

(event OnComponentEndOverlap(Collision)
  (params (OverlappedComponent :type Primitive%20Component%20Object%20Reference) (OtherActor :type Actor%20Object%20Reference) (OtherComp :type Primitive%20Component%20Object%20Reference) (OtherBodyIndex :type Integer))
  (Utilities|Casting|CastToThirdPersonCharacter OtherActor)
  (Input|DisableInput (Game|GetPlayerController 0)))

(event EventBeginPlay)

(event Collision|EventActorBeginOverlap
  (params (OtherActor :type Actor%20Object%20Reference)))

(event EventTick
  (params (DeltaSeconds :type Float%20%28single-precision%29)))

(event Input|KeyboardEvents|F
  (params (Key :type Key%20Structure :default "None"))
  (:Pressed
    (bind _asthird_person_game_mode (Utilities|Casting|CastToThirdPersonGameMode (Game|GetGameMode)))
    (bind _result (Math|Integer|IncrementInt (Variables|/Game/ThirdPersonBP/Blueprints/ThirdPersonGameMode.ThirdPersonGameMode_C|GetTotal_Torsos _asthird_person_game_mode))
      (:%20%20
        (Variables|/Game/ThirdPersonBP/Blueprints/ThirdPersonGameMode.ThirdPersonGameMode_C|SetTorsos_Collected _asthird_person_game_mode _result)
        (Variables|/Game/ThirdPersonBP/Blueprints/ThirdPersonGameMode.ThirdPersonGameMode_C|SetTotal_Torsos _asthird_person_game_mode _result)
        (bind _returnvalue (Actor|GetActorOfClass "/Game/NEOVOLUTION/Blueprints/Puzzles/Statues/StatuesWindow_BP.StatuesWindow_BP_C"))
        (Variables|/Game/NEOVOLUTION/Blueprints/Puzzles/Statues/StatuesWindow_BP.StatuesWindow_BP_C|SettorsosCollected _returnvalue true)
        (bind _returnvalue_2 (UserInterface|CreateWidget "/Game/NEOVOLUTION/Blueprints/Widgets/UI/Statues/Torso_Collectable_Widget.Torso_Collectable_Widget_C"))
        (UserInterface|Viewport|AddtoViewport _returnvalue_2 0)
        (Audio|PlaySoundatLocation "/Game/NEOVOLUTION/Music_Sounds/Puzzles/Item_Pickup/itemsCue.itemsCue" (Transformation|GetActorLocation) "0, 0, 0" 1.0 1.0 0.0 0 0 0)
        (Game|SpawnActorfromClass "/Game/NEOVOLUTION/Blueprints/Puzzles/Statues/Torso_Spawnable_BP.Torso_Spawnable_BP_C" (Math|Transform|MakeTransform "1270.000000,7980.000000,144.000000" "0,180.000000, 0" "1,1,1") "Undefined" 0 0)
        (Actor|DestroyActor)))))

(fn ConstructionScript)