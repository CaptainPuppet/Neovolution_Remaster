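; Collectable statue-arm pickup for the puzzles, picked up by pressing F while the player is in range.
; Its Collision overlap enables actor input for the ThirdPersonCharacter and disables it on exit.
; Pressing F increments ArmCollectablesLeft on the ThirdPersonGameMode, copies the count into TotalArms, adds an Arms_Collectable_Widget to the viewport and destroys the actor.
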(event OnComponentBeginOverlap(Collision)
  (params (OverlappedComponent :type Primitive%20Component%20Object%20Reference) (OtherActor :type Actor%20Object%20Reference) (OtherComp :type Primitive%20Component%20Object%20Reference) (OtherBodyIndex :type Integer) (bFromSweep :type Boolean) (SweepResult :type Hit%20Result%20Structure%20%28by%20ref%29))
  (Utilities|Casting|CastToThirdPersonCharacter OtherActor)
  (Input|EnableInput (Game|GetPlayerController 0)))

(event OnComponentEndOverlap(Collision)
  (params (OverlappedComponent :type Primitive%20Component%20Object%20Reference) (OtherActor :type Actor%20Object%20Reference) (OtherComp :type Primitive%20Component%20Object%20Reference) (OtherBodyIndex :type Integer))
  (Utilities|Casting|CastToThirdPersonCharacter OtherActor)
  (Input|DisableInput (Game|GetPlayerController 0)))

(event EventBeginPlay)

(event Collision|EventActorBeginOverlap
  (params (OtherActor :type Actor%20Object%20Reference)))

(event EventTick
  (params (DeltaSeconds :type Float%20%28single-precision%29)))

(event Input|KeyboardEvents|F
  (params (Key :type Key%20Structure :default "None"))
  (:Pressed
    (bind _asthird_person_game_mode (Utilities|Casting|CastToThirdPersonGameMode (Game|GetGameMode)))
    (bind _result (Math|Integer|IncrementInt (Variables|/Game/ThirdPersonBP/Blueprints/ThirdPersonGameMode.ThirdPersonGameMode_C|GetArm_Collectables_Left _asthird_person_game_mode))
      (:%20%20
        (Variables|/Game/ThirdPersonBP/Blueprints/ThirdPersonGameMode.ThirdPersonGameMode_C|SetArm_Collectables_Left _asthird_person_game_mode _result)
        (Variables|/Game/ThirdPersonBP/Blueprints/ThirdPersonGameMode.ThirdPersonGameMode_C|SetTotal_Arms _asthird_person_game_mode _result)
        (bind _returnvalue (UserInterface|CreateWidget "/Game/NEOVOLUTION/Blueprints/Widgets/UI/Arms_Collectable_Widget.Arms_Collectable_Widget_C"))
        (UserInterface|Viewport|AddtoViewport _returnvalue 0)
        (Actor|DestroyActor)))))

(fn ConstructionScript)