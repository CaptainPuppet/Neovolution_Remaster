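; Puzzle door for the statues puzzle that slides open for the player once all arm, foot, torso and head collection flags are true.
; Entering DoorTrigger as the ThirdPersonCharacter checks the flags and plays the OpenCloseDoor timeline, which drives the mesh's relative X and Y while keeping Z.
; Leaving the trigger reverses the timeline without checking the flags.
; The flags are only read here, and UpdateLight is an empty stub.
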(event OnComponentBeginOverlap(DoorTrigger)
  (params (OverlappedComponent :type Primitive%20Component%20Object%20Reference) (OtherActor :type Actor%20Object%20Reference) (OtherComp :type Primitive%20Component%20Object%20Reference) (OtherBodyIndex :type Integer) (bFromSweep :type Boolean) (SweepResult :type Hit%20Result%20Structure%20%28by%20ref%29))
  (if (and (and (Variables|Default|GetarmsCollected) (Variables|Default|GetfeetCollected)) (and (Variables|Default|GettorsosCollected) (Variables|Default|GetheadsCollected)))
    (Utilities|Casting|CastToThirdPersonCharacter OtherActor)
    (bind (_direction _ejey _ejex) (Timeline|Open/CloseDoor Play)
      (:Update
        (Transformation|SetRelativeLocation (Variables|Default|GetDoorMesh) (Math|Vector|MakeVector _ejex _ejey (.z (Variables|/Script/Engine.SceneComponent|GetRelativeLocation (Variables|Default|GetDoorMesh)))) false false)))))

(event OnComponentEndOverlap(DoorTrigger)
  (params (OverlappedComponent :type Primitive%20Component%20Object%20Reference) (OtherActor :type Actor%20Object%20Reference) (OtherComp :type Primitive%20Component%20Object%20Reference) (OtherBodyIndex :type Integer))
  (Utilities|Casting|CastToThirdPersonCharacter OtherActor)
  (bind (_direction _ejey _ejex) (Timeline|Open/CloseDoor Reverse)
    (:Update
      (Transformation|SetRelativeLocation (Variables|Default|GetDoorMesh) (Math|Vector|MakeVector _ejex _ejey (.z (Variables|/Script/Engine.SceneComponent|GetRelativeLocation (Variables|Default|GetDoorMesh)))) false false))))

(event EventBeginPlay)

(event Collision|EventActorBeginOverlap
  (params (OtherActor :type Actor%20Object%20Reference)))

(event EventTick
  (params (DeltaSeconds :type Float%20%28single-precision%29)))

(fn ConstructionScript)

(fn UpdateLight)